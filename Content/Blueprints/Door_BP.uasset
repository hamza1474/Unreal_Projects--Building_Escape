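; Door_BP is a door actor that swings open and closed in response to open and close requests from an OpenDoor component.
; It stores its starting rotation on BeginPlay, then a timeline's OpenAngle track adds yaw to that rotation each update.
; An event track on the timeline plays a door lock sound at the door's location, and close requests reverse the timeline.
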(event OnOpenRequest(OpenDoor)
  (bind _openangle (Timeline|Timeline_0 Play)
    (:Update
      (Transformation|SetActorRotation (Math|Rotator|CombineRotators (Math|Rotator|MakeRotator 0.0 0.0 _openangle) (Variables|Default|GetInitialRotation))))
    (:SoundTime
      (Audio|PlaySoundatLocation "/Game/Audio/51_3_door_lock_wav.51_3_door_lock_wav" (Transformation|GetActorLocation) "0, 0, 0" 1.0 1.0 0.0 0 0 0))))

(event OnCloseRequest(OpenDoor)
  (bind _openangle (Timeline|Timeline_0 Reverse)
    (:Update
      (Transformation|SetActorRotation (Math|Rotator|CombineRotators (Math|Rotator|MakeRotator 0.0 0.0 _openangle) (Variables|Default|GetInitialRotation))))
    (:SoundTime
      (Audio|PlaySoundatLocation "/Game/Audio/51_3_door_lock_wav.51_3_door_lock_wav" (Transformation|GetActorLocation) "0, 0, 0" 1.0 1.0 0.0 0 0 0))))

(event EventBeginPlay
  (Variables|Default|SetInitialRotation (Transformation|GetActorRotation)))

(fn ConstructionScript)